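; Player character Blueprint for a shooter that creates the player HUD and tracks sprint, aim and reload input.
; BeginPlay creates a BP_PlayerHUD widget and adds it to the viewport.
; The AnimationBinding graph sets Sprinting, Aiming and Reloading flags while their inputs are held, with Aim also driving IsTargeting.
; The graphs only set these flags and contain no movement, weapon or reload logic.
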(event EventBeginPlay
  (bind _returnvalue (UserInterface|CreateWidget "/Game/Blueprints/UI/BP_PlayerHUD.BP_PlayerHUD_C"))
  (UserInterface|Viewport|AddtoViewport _returnvalue 0))

(event Collision|EventActorBeginOverlap
  (params (OtherActor :type Actor%20Object%20Reference)))

(event EventTick
  (params (DeltaSeconds :type Float%20%28single-precision%29)))

(event Input|ActionEvents|InputActionAim
  (params (Key :type Key%20Structure))
  (:Pressed
    (Variables|Default|SetAiming true)
    (Variables|Default|SetbIsTargeting true))
  (:Released
    (Variables|Default|SetAiming false)
    (Variables|Default|SetbIsTargeting false)))

(event Input|ActionEvents|InputActionReload
  (params (Key :type Key%20Structure))
  (:Pressed
    (Variables|Default|SetReloading true))
  (:Released
    (Variables|Default|SetReloading false)))

(event Input|ActionEvents|InputActionSprint
  (params (Key :type Key%20Structure))
  (:Pressed
    (Variables|Default|SetSprinting true))
  (:Released
    (Variables|Default|SetSprinting false)))

(fn ConstructionScript)